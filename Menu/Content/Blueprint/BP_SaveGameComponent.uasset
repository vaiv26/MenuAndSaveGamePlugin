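; Actor component that saves and restores its owner's transform, stored as the player transform, through a BP_SaveGame slot.
; SaveGame creates the save object when the validity check fails, copies in the owner's transform and writes it to the slot.
; LoadGame moves the owner to the stored transform, or calls SaveGame when no save exists.
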(event EventBeginPlay)

(event EventTick
  (params (DeltaSeconds :type Float%20%28single-precision%29)))

(fn SaveGame
  (Utilities|FlowControl|Sequence
    (:then_0
      (Utilities|IsValid 0
        (:Is%20Not%20Valid
          (bind _returnvalue (SaveGame|CreateSaveGameObject "/Menu/Blueprint/BP_SaveGame.BP_SaveGame_C"))
          (Variables|Default|SetSaveGameRef _returnvalue))))
    (:then_1
      (Variables|/Menu/Blueprint/BP_SaveGame.BP_SaveGame_C|SetPlayerTransaform (Variables|Default|GetSaveGameRef) (Transformation|GetActorTransform (Components|GetOwner))))
    (:then_2
      (SaveGame|SaveGametoSlot (Variables|Default|GetSaveGameRef) (Variables|Default|GetSaveGameSlot)))))

(fn LoadGame
  (bind _returnvalue (SaveGame|DoesSaveGameExist (Variables|Default|GetSaveGameSlot)))
  (if _returnvalue
    (bind _returnvalue_2 (SaveGame|LoadGamefromSlot (Variables|Default|GetSaveGameSlot)))
    (bind _asbp_save_game (Utilities|Casting|CastToBP_SaveGame _returnvalue_2))
    (Transformation|SetActorTransform (Components|GetOwner) (Variables|/Menu/Blueprint/BP_SaveGame.BP_SaveGame_C|GetPlayerTransaform _asbp_save_game))
    (else
      (CallFunction|SaveGame))))